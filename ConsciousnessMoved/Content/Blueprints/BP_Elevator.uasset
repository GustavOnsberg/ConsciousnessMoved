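; Elevator actor that opens and closes its doors in response to linked activators; only the Waiting state is implemented, with no travel logic.
; Each Tick polls the Activators array to set Active, requiring either any or all of them according to RequireAllActivators.
; While Waiting, Active ramps a clamped Openness value up or down, positioning door halves, or raising roof and frame parts, per the StartPointSettings flags.
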(event EventBeginPlay)

(event Collision|EventActorBeginOverlap
  (params (OtherActor :type Actor%20Object%20Reference)))

(event EventTick
  (params (DeltaSeconds :type Float%20%28single-precision%29))
  (bind _speed (Variables|Default|GetSpeed))
  (bind _startpointsettings (Variables|Default|GetStartPointSettings))
  (bind _floor_y (Variables|Default|GetFloor-Y))
  (bind _requireallactivators (Variables|Default|GetRequireAllActivators))
  (bind _door_x (Variables|Default|GetDoor+X))
  (bind _door_y (Variables|Default|GetDoor+Y))
  (bind _door_x_2 (Variables|Default|GetDoor-X))
  (bind _returnvalue (* DeltaSeconds _speed))
  (bind _relativelocation (Variables|/Script/Engine.SceneComponent|GetRelativeLocation _door_x_2))
  (bind _relativelocation_2 (Variables|/Script/Engine.SceneComponent|GetRelativeLocation _door_y))
  (bind _relativelocation_3 (Variables|/Script/Engine.SceneComponent|GetRelativeLocation _floor_y))
  (bind _relativelocation_4 (Variables|/Script/Engine.SceneComponent|GetRelativeLocation _door_x))
  (Utilities|FlowControl|Sequence
    (:then_0
      (bind _array_element (Utilities|Array|ForEachLoopwithBreak (Variables|Default|GetActivators) :!label _label)
        (:LoopBody
          (if (Variables|/Game/Blueprints/BP_Activator.BP_Activator_C|GetActive _array_element)
            (Variables|Default|SetActive true)
            (if (not _requireallactivators)
              (goto _label Break))
            (else
              (Variables|Default|SetActive false)
              (if _requireallactivators
                (goto _label Break)))))))
    (:then_1
      (switch Utilities|FlowControl|Switch|SwitchonElevatorStatus (Variables|Default|GetStatus)
        (:NewEnumerator0
          (if (Variables|Default|GetActive)
            (Variables|Default|SetOpenness (Math|Float|Clamp(Float) (+ (Variables|Default|GetOpenness) _returnvalue)))
            (else
              (Variables|Default|SetOpenness (Math|Float|Clamp(Float) (- (Variables|Default|GetOpenness) _returnvalue)))))
          (if (.open-y _startpointsettings)
            (Transformation|SetRelativeLocation (Variables|Default|GetDoor-Y_L) (Math|Vector|MakeVector (* (Variables|Default|GetOpenness) 1e+02) 0.0 0.0) false false)
            (Transformation|SetRelativeLocation (Variables|Default|GetDoor-Y_R) (Math|Vector|MakeVector (- 0.0 (* (Variables|Default|GetOpenness) 1e+02)) 0.0 0.0) false false))
          (if (.open+x _startpointsettings)
            (Transformation|SetRelativeLocation (Variables|Default|GetDoor+X_L) (Math|Vector|MakeVector (* (Variables|Default|GetOpenness) 1e+02) 0.0 0.0) false false)
            (Transformation|SetRelativeLocation (Variables|Default|GetDoor+X_R) (Math|Vector|MakeVector (- 0.0 (* (Variables|Default|GetOpenness) 1e+02)) 0.0 0.0) false false))
          (if (.open+y _startpointsettings)
            (Transformation|SetRelativeLocation (Variables|Default|GetDoor+Y_L) (Math|Vector|MakeVector (* (Variables|Default|GetOpenness) 1e+02) 0.0 0.0) false false)
            (Transformation|SetRelativeLocation (Variables|Default|GetDoor+Y_R) (Math|Vector|MakeVector (- 0.0 (* (Variables|Default|GetOpenness) 1e+02)) 0.0 0.0) false false))
          (if (.open-x _startpointsettings)
            (Transformation|SetRelativeLocation (Variables|Default|GetDoor-X_L) (Math|Vector|MakeVector 0.0 0.0 0.0) false false)
            (Transformation|SetRelativeLocation (Variables|Default|GetDoor-X_R) (Math|Vector|MakeVector 0.0 0.0 0.0) false false))
          (if (.opentop _startpointsettings)
            (Transformation|SetRelativeLocation (Variables|Default|GetRoof) (Math|Vector|MakeVector 0.0 0.0 (* (Variables|Default|GetOpenness) 2.5e+02)) false false)
            (Transformation|SetRelativeLocation _floor_y (Math|Vector|MakeVector (.x _relativelocation_3) (.y _relativelocation_3) (* (Variables|Default|GetOpenness) 3.8e+02)) false false)
            (Transformation|SetRelativeLocation _door_x (Math|Vector|MakeVector (.x _relativelocation_4) (.y _relativelocation_4) (* (Variables|Default|GetOpenness) 3.8e+02)) false false)
            (Transformation|SetRelativeLocation _door_y (Math|Vector|MakeVector (.x _relativelocation_2) (.y _relativelocation_2) (* (Variables|Default|GetOpenness) 3.8e+02)) false false)
            (Transformation|SetRelativeLocation _door_x_2 (Math|Vector|MakeVector (.x _relativelocation) (.y _relativelocation) (* (Variables|Default|GetOpenness) 3.8e+02)) false false)))))))

(fn ConstructionScript)