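; Player controller for a body-possession mechanic, creating the HUD and remembering the starting BP_Default_Character as the default host.
; An input action returns the player to that host, handing the currently possessed pawn to the host's controller.
; Die repossesses the host, moves it above the last elevator, unloads and reloads the current streamed level, and changes the elevator's status.
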(event EventBeginPlay
  (bind _returnvalue (UserInterface|CreateWidget "/Game/UI/UI_HUD.UI_HUD_C"))
  (UserInterface|Viewport|AddtoViewport _returnvalue 0)
  (bind _asbp_default_character (Utilities|Casting|CastToBP_Default_Character (Pawn|GetControlledPawn)))
  (Variables|Default|SetDefaultHost _asbp_default_character))

(event EventTick
  (params (DeltaSeconds :type Float%20%28single-precision%29)))

(event Custom|Die
  (bind _currentlevel (Variables|Default|GetCurrentLevel))
  (bind _lastelevator (Variables|Default|GetLastElevator))
  (Pawn|Possess (Variables|Default|GetDefaultHost))
  (Transformation|SetActorLocation (Variables|Default|GetDefaultHost) (+ (Transformation|GetActorLocation _lastelevator) "0, 0,200.000000") false false)
  (Game|UnloadStreamLevel(byName) _currentlevel)
  (Game|LoadStreamLevel(byName) _currentlevel true)
  (Variables|/Game/Blueprints/LevelBuild/BP_Elevator.BP_Elevator_C|SetStatus _lastelevator "NewEnumerator2"))

(event Input|ActionEvents|InputActionReturntodefaulthost
  (params (Key :type Key%20Structure))
  (bind _defaulthost (Variables|Default|GetDefaultHost))
  (:Pressed
    (if (!= (Pawn|GetControlledPawn) (Variables|Default|GetDefaultHost))
      (Pawn|Possess (Pawn|GetController _defaulthost) (Pawn|GetControlledPawn))
      (Pawn|Possess _defaulthost))))

(fn ConstructionScript)