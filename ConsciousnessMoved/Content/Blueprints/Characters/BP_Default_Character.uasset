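; BP_Default_Character is a character Blueprint whose only active logic is a Die event that handles death and respawn.
; Die reads the current level name and start location from BP_PlayerController, unloads and reloads that streamed level, then moves the character back to the start.
; Resetting through level streaming keeps the same character actor rather than respawning it.
; BeginPlay, overlap, Tick and the construction script add no behavior of their own.
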(event Custom|Die
  (bind _asbp_player_controller (Utilities|Casting|CastToBP_PlayerController (Pawn|GetController)))
  (Game|UnloadStreamLevel(byName) (Variables|/Game/Blueprints/BP_PlayerController.BP_PlayerController_C|GetCurrentLevel _asbp_player_controller))
  (Game|LoadStreamLevel(byName) (Variables|/Game/Blueprints/BP_PlayerController.BP_PlayerController_C|GetCurrentLevel _asbp_player_controller) true)
  (Transformation|SetActorLocation (Variables|/Game/Blueprints/BP_PlayerController.BP_PlayerController_C|GetCurrentLevelStart _asbp_player_controller) false false))

(event EventBeginPlay
  (|CallParentFunction) ; This node is disabled and will not be called.\nDrag off pins to build functionality.
)

(event Collision|EventActorBeginOverlap
  (params (OtherActor :type Actor%20Object%20Reference))
  (|CallParentFunction OtherActor) ; This node is disabled and will not be called.\nDrag off pins to build functionality.
)

(event EventTick
  (params (DeltaSeconds :type Float%20%28single-precision%29))
  (|CallParentFunction DeltaSeconds) ; This node is disabled and will not be called.\nDrag off pins to build functionality.
)

(fn ConstructionScript
  (|CallParentFunction))