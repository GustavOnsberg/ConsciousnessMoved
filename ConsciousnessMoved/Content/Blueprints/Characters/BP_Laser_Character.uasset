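; BP_Laser_Character is a character that emits a laser beam which locks onto BP_LaserReciver actors.
; Each tick it line-traces from LaserOrigin to a target location, stretches the beam particle to the impact point, and registers itself with any receiver hit.
; A hit receiver pulls the next target location to just above it; otherwise the laser aims far forward.
; SecondAction breaks the lock by resetting the aim forward.
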(event EventBeginPlay
  (|CallParentFunction) ; This node is disabled and will not be called.\nDrag off pins to build functionality.
)

(event Collision|EventActorBeginOverlap
  (params (OtherActor :type Actor%20Object%20Reference))
  (|CallParentFunction OtherActor) ; This node is disabled and will not be called.\nDrag off pins to build functionality.
)

(event EventTick
  (params (DeltaSeconds :type Float%20%28single-precision%29))
  (bind _particlesystem (Variables|Default|GetParticleSystem))
  (bind _laserorigin (Variables|Default|GetLaserOrigin))
  (|CallParentFunction DeltaSeconds)
  (Utilities|FlowControl|Sequence
    (:then_0
      (bind _outhit (Collision|LineTraceByChannel (Transformation|GetWorldLocation (Variables|Default|GetLaserOrigin)) (Variables|Default|GetTargetLocation) "TraceTypeQuery1" false 0 "None"))
      (bind _asbp_laser_reciver (Utilities|Casting|CastToBP_LaserReciver (.HitActor (Collision|BreakHitResult _outhit)))
        (:then
          (Variables|Default|SetLasarTarget _asbp_laser_reciver)
          (Utilities|Array|AddUnique (Variables|/Game/Blueprints/LevelBuild/BP_LaserReciver.BP_LaserReciver_C|GetLaserOrigins _asbp_laser_reciver) self))
        (:CastFailed
          (Variables|Default|SetLasarTarget 0)))
      (Class|ParticleSystemComponent|SetBeamSourcePoint _particlesystem 0 (Transformation|GetWorldLocation _particlesystem))
      (Class|ParticleSystemComponent|SetBeamTargetPoint _particlesystem 0 (.ImpactPoint (Collision|BreakHitResult _outhit))))
    (:then_1
      (if (!= (Variables|Default|GetLasarTarget) 0)
        (Variables|Default|SetFocusOnTarget true)
        (else
          (Variables|Default|SetFocusOnTarget false))))
    (:then_2
      (if (Variables|Default|GetFocusOnTarget)
        (Variables|Default|SetTargetLocation (+ (Transformation|GetActorLocation (Variables|Default|GetLasarTarget)) (* (Transformation|GetActorUpVector (Variables|Default|GetLasarTarget)) 8e+01)))
        (else
          (Variables|Default|SetTargetLocation (+ (Transformation|GetWorldLocation _laserorigin) (* (Math|Vector|GetForwardVector _laserorigin) 5e+05))))))))

(event Input|ActionEvents|InputActionSecondAction
  (params (Key :type Key%20Structure))
  (bind _lasartarget (Variables|Default|GetLasarTarget))
  (bind _laserorigin (Variables|Default|GetLaserOrigin))
  (:Pressed
    (Variables|Default|SetFocusOnTarget false)
    (if (Variables|Default|GetFocusOnTarget)
      (Variables|Default|SetTargetLocation (+ (Transformation|GetActorLocation _lasartarget) (* (Transformation|GetActorUpVector _lasartarget) 8e+01)))
      (else
        (Variables|Default|SetTargetLocation (+ (Transformation|GetWorldLocation _laserorigin) (* (Math|Vector|GetForwardVector _laserorigin) 5e+05)))))))

(fn ConstructionScript
  (|CallParentFunction))