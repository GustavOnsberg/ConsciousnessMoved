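; Character Blueprint that teleports to the spot the camera aims at when SecondAction is pressed.
; Each Tick, a Visibility line trace from the camera places TeleportTestCollision at the hit, nudging it off flat floors or ceilings using the impact normal.
; TeleportBlockingObjects only switches the debug print between the normal's Z and "Can not teleport".
; The input moves the actor to the test collision without checking that array.
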(event EventBeginPlay
  (|CallParentFunction) ; This node is disabled and will not be called.\nDrag off pins to build functionality.
)

(event Collision|EventActorBeginOverlap
  (params (OtherActor :type Actor%20Object%20Reference))
  (|CallParentFunction OtherActor) ; This node is disabled and will not be called.\nDrag off pins to build functionality.
)

(event EventTick
  (params (DeltaSeconds :type Float%20%28single-precision%29))
  (bind _teleporttestcollision (Variables|Default|GetTeleportTestCollision))
  (bind _camera (Variables|Default|GetCamera))
  (bind _returnvalue (Transformation|GetWorldLocation _camera))
  (|CallParentFunction DeltaSeconds)
  (bind _outhit (Collision|LineTraceByChannel _returnvalue (+ _returnvalue (* (Math|Vector|GetForwardVector _camera) 1e+04)) "TraceTypeQuery1" false 0 "None"))
  (if (== (.Z (Math|Vector|BreakVector (.ImpactNormal (Collision|BreakHitResult _outhit)))) 1.0)
    (Transformation|SetWorldLocation _teleporttestcollision (+ (.Location (Collision|BreakHitResult _outhit)) "0, 0,100.000000") false false)
    (elif (== (.Z (Math|Vector|BreakVector (.ImpactNormal (Collision|BreakHitResult _outhit)))) -1.0)
      (Transformation|SetWorldLocation _teleporttestcollision (- (.Location (Collision|BreakHitResult _outhit)) "0, 0,100.000000") false false)
      (else
        (Transformation|SetWorldLocation _teleporttestcollision (.Location (Collision|BreakHitResult _outhit)) false false))))
  (if (== (Utilities|Array|Length (Variables|Default|GetTeleportBlockingObjects)) 0)
    (Development|PrintString (Utilities|String|ToString(Float) (.Z (Math|Vector|BreakVector (.ImpactNormal (Collision|BreakHitResult _outhit))))) true true "(R=0.000000,G=1.000000,B=0.000000,A=1.000000)")
    (else
      (Development|PrintString "Can not teleport" true true "(R=1.000000,G=0.000000,B=0.000000,A=1.000000)"))))

(event Input|ActionEvents|InputActionSecondAction
  (params (Key :type Key%20Structure))
  (:Pressed
    (Transformation|SetActorLocation (Transformation|GetWorldLocation (Variables|Default|GetTeleportTestCollision)) false false)))

(fn ConstructionScript
  (|CallParentFunction))