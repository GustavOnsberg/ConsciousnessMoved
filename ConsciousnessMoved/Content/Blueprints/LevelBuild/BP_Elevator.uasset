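; One-way elevator that opens when its Activators are active and carries the player along a Route spline.
; Tick runs a state machine: wait until the player is inside and closed, ease up to speed along the spline, then open until the player leaves.
; Openness animates the doors, roof or floor panels chosen by start or end point settings.
; On arrival, a player missing from PlayerNearField is teleported to the car.
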(event EventBeginPlay
  (Variables|Default|SetSettingsToUse (Variables|Default|GetStartPointSettings)))

(event Collision|EventActorBeginOverlap
  (params (OtherActor :type Actor%20Object%20Reference)))

(event EventTick
  (params (DeltaSeconds :type Float%20%28single-precision%29))
  (bind _returnvalue (Utilities|Time|GetWorldDeltaSeconds))
  (bind _floor_y (Variables|Default|GetFloor-Y))
  (bind _floor_x (Variables|Default|GetFloor+X))
  (bind _speed (Variables|Default|GetSpeed))
  (bind _floor_y_2 (Variables|Default|GetFloor+Y))
  (bind _requireallactivators (Variables|Default|GetRequireAllActivators))
  (bind _floor_x_2 (Variables|Default|GetFloor-X))
  (bind _route (Variables|Default|GetRoute))
  (bind _returnvalue_2 (* DeltaSeconds _speed))
  (bind _spline (Variables|/Game/Blueprints/LevelBuild/BP_ElevatorRoute.BP_ElevatorRoute_C|GetSpline _route))
  (bind _relativelocation (Variables|/Script/Engine.SceneComponent|GetRelativeLocation _floor_y))
  (bind _relativelocation_2 (Variables|/Script/Engine.SceneComponent|GetRelativeLocation _floor_x))
  (bind _relativelocation_3 (Variables|/Script/Engine.SceneComponent|GetRelativeLocation _floor_y_2))
  (bind _relativelocation_4 (Variables|/Script/Engine.SceneComponent|GetRelativeLocation _floor_x_2))
  (bind _returnvalue_3 (Spline|GetSplineLength _spline))
  (Utilities|FlowControl|Sequence
    (:then_0
      (bind _array_element (Utilities|Array|ForEachLoopwithBreak (Variables|Default|GetActivators) :!label _label)
        (:LoopBody
          (if (Variables|/Game/Blueprints/BP_Activator.BP_Activator_C|GetActive _array_element)
            (Variables|Default|SetActive true)
            (if (not _requireallactivators)
              (goto _label Break))
            (else
              (Variables|Default|SetActive false)
              (if _requireallactivators
                (goto _label Break)))))))
    (:then_1
      (switch Utilities|FlowControl|Switch|SwitchonElevatorStatus (Variables|Default|GetStatus)
        (:NewEnumerator0
          (Utilities|FlowControl|Sequence
            (:then_0
              (if (and (Variables|Default|GetActive) (not (Variables|Default|GetPlayerIn)))
                (Variables|Default|SetOpenness (Math|Float|Clamp(Float) (+ (Variables|Default|GetOpenness) _returnvalue_2)) :!label _label_2)
                (else
                  (Variables|Default|SetOpenness (Math|Float|Clamp(Float) (- (Variables|Default|GetOpenness) _returnvalue_2)) :!label _label_3)))
              (if (.Open-Y (Utilities|Struct|BreakElevatorSettings (Variables|Default|GetSettingsToUse)))
                (Transformation|SetRelativeLocation (Variables|Default|GetDoor-Y_L) (Math|Vector|MakeVector (* (Variables|Default|GetOpenness) 1e+02) 0.0 0.0) false false)
                (Transformation|SetRelativeLocation (Variables|Default|GetDoor-Y_R) (Math|Vector|MakeVector (- 0.0 (* (Variables|Default|GetOpenness) 1e+02)) 0.0 0.0) false false))
              (if (.Open+X (Utilities|Struct|BreakElevatorSettings (Variables|Default|GetSettingsToUse)))
                (Transformation|SetRelativeLocation (Variables|Default|GetDoor+X_L) (Math|Vector|MakeVector (* (Variables|Default|GetOpenness) 1e+02) 0.0 0.0) false false)
                (Transformation|SetRelativeLocation (Variables|Default|GetDoor+X_R) (Math|Vector|MakeVector (- 0.0 (* (Variables|Default|GetOpenness) 1e+02)) 0.0 0.0) false false))
              (if (.Open+Y (Utilities|Struct|BreakElevatorSettings (Variables|Default|GetSettingsToUse)))
                (Transformation|SetRelativeLocation (Variables|Default|GetDoor+Y_L) (Math|Vector|MakeVector (* (Variables|Default|GetOpenness) 1e+02) 0.0 0.0) false false)
                (Transformation|SetRelativeLocation (Variables|Default|GetDoor+Y_R) (Math|Vector|MakeVector (- 0.0 (* (Variables|Default|GetOpenness) 1e+02)) 0.0 0.0) false false))
              (if (.Open-X (Utilities|Struct|BreakElevatorSettings (Variables|Default|GetSettingsToUse)))
                (Transformation|SetRelativeLocation (Variables|Default|GetDoor-X_L) (Math|Vector|MakeVector (* (Variables|Default|GetOpenness) 1e+02) 0.0 0.0) false false)
                (Transformation|SetRelativeLocation (Variables|Default|GetDoor-X_R) (Math|Vector|MakeVector (- 0.0 (* (Variables|Default|GetOpenness) 1e+02)) 0.0 0.0) false false))
              (if (.OpenTop (Utilities|Struct|BreakElevatorSettings (Variables|Default|GetSettingsToUse)))
                (Transformation|SetRelativeLocation (Variables|Default|GetRoof) (Math|Vector|MakeVector 0.0 0.0 (* (Variables|Default|GetOpenness) 3.2e+02)) false false)
                (Transformation|SetRelativeLocation _floor_y (Math|Vector|MakeVector (.x _relativelocation) (.y _relativelocation) (* (Variables|Default|GetOpenness) 3.8e+02)) false false)
                (Transformation|SetRelativeLocation _floor_x (Math|Vector|MakeVector (.x _relativelocation_2) (.y _relativelocation_2) (* (Variables|Default|GetOpenness) 3.8e+02)) false false)
                (Transformation|SetRelativeLocation _floor_y_2 (Math|Vector|MakeVector (.x _relativelocation_3) (.y _relativelocation_3) (* (Variables|Default|GetOpenness) 3.8e+02)) false false)
                (Transformation|SetRelativeLocation _floor_x_2 (Math|Vector|MakeVector (.x _relativelocation_4) (.y _relativelocation_4) (* (Variables|Default|GetOpenness) 3.8e+02)) false false)
                (elif (.OpenBottom (Utilities|Struct|BreakElevatorSettings (Variables|Default|GetSettingsToUse)))
                  (Transformation|SetRelativeRotation (Variables|Default|GetFloor-Y) (Math|Rotator|MakeRotator (* (Variables|Default|GetOpenness) 9e+01) 0.0 0.0) false false)
                  (Transformation|SetRelativeRotation (Variables|Default|GetFloor+X) (Math|Rotator|MakeRotator (* (Variables|Default|GetOpenness) 9e+01) 0.0 9e+01) false false)
                  (Transformation|SetRelativeRotation (Variables|Default|GetFloor+Y) (Math|Rotator|MakeRotator (* (Variables|Default|GetOpenness) 9e+01) 0.0 1.8e+02) false false)
                  (Transformation|SetRelativeRotation (Variables|Default|GetFloor-X) (Math|Rotator|MakeRotator (* (Variables|Default|GetOpenness) 9e+01) 0.0 -9e+01) false false))))
            (:then_1
              (if (> (Utilities|Array|Length (Collision|GetOverlappingActors (Variables|Default|GetTrigger) "/Game/Blueprints/Characters/BP_Default_Character.BP_Default_Character_C" :!class /Script/Engine.PrimitiveComponent)) 0)
                (Variables|Default|SetPlayerIn true)
                (if (<= (Variables|Default|GetOpenness) 0.0)
                  (Variables|Default|SetStatus "NewEnumerator1")
                  (Variables|Default|SetSettingsToUse (Variables|Default|GetEndPointSettings)))
                (else
                  (Variables|Default|SetPlayerIn false))))))
        (:NewEnumerator1
          (Variables|Default|SetMovingSpeed (Math|Float|Lerp (Variables|Default|GetMovingSpeed) (Variables|Default|GetMovementSpeed) _returnvalue))
          (if (< (+ (Variables|Default|GetMovedDistance) (* _returnvalue (Variables|Default|GetMovingSpeed))) _returnvalue_3)
            (Transformation|SetActorLocation (- (Spline|GetLocationatDistanceAlongSpline _spline (+ (Variables|Default|GetMovedDistance) (* _returnvalue (Variables|Default|GetMovingSpeed))) "World") "0, 0,200.000000") false false)
            (Variables|Default|SetMovedDistance (+ (Variables|Default|GetMovedDistance) (* _returnvalue (Variables|Default|GetMovingSpeed))))
            (else
              (Transformation|SetActorLocation (- (Spline|GetLocationatDistanceAlongSpline _spline _returnvalue_3 "World") "0, 0,200.000000") false false)
              (Variables|Default|SetStatus "NewEnumerator2")
              (if (not (> (Utilities|Array|Length (Collision|GetOverlappingActors (Variables|Default|GetPlayerNearField) "/Game/Blueprints/Characters/BP_Default_Character.BP_Default_Character_C" :!class /Script/Engine.PrimitiveComponent)) 0))
                (Transformation|SetActorLocation (Game|Player|GetPlayerPawn 0) (+ (Transformation|GetActorLocation) "0, 0,200.000000") false true)))))
        (:NewEnumerator2
          (if (> (Utilities|Array|Length (Collision|GetOverlappingActors (Variables|Default|GetPlayerNearField) "/Game/Blueprints/Characters/BP_Default_Character.BP_Default_Character_C" :!class /Script/Engine.PrimitiveComponent)) 0)
            (goto _label_2)
            (elif (> (Variables|Default|GetOpenness) 0.0)
              (goto _label_3)
              (else
                (Variables|Default|SetStatus "NewEnumerator3")))))))))

(fn ConstructionScript)