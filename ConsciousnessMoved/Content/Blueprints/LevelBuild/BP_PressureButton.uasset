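; BP_PressureButton is a level-building pressure plate that activates while a character or heavy cube rests on it.
; Each Tick polls the Cylinder component for overlapping BP_BaseCharacter or BP_HeavyCube actors and sets the Active flag accordingly, rather than using overlap events.
; The same check slides the Button component down or up at Speed scaled by delta time, clamping its relative height between pressed and raised limits.
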(event EventBeginPlay
  (|CallParentFunction) ; This node is disabled and will not be called.\nDrag off pins to build functionality.
)

(event Collision|EventActorBeginOverlap
  (params (OtherActor :type Actor%20Object%20Reference))
  (|CallParentFunction OtherActor) ; This node is disabled and will not be called.\nDrag off pins to build functionality.
)

(event EventTick
  (params (DeltaSeconds :type Float%20%28single-precision%29))
  (bind _button (Variables|Default|GetButton))
  (bind _speed (Variables|Default|GetSpeed))
  (bind _returnvalue (* DeltaSeconds _speed))
  (bind _relativelocation (Variables|/Script/Engine.SceneComponent|GetRelativeLocation _button))
  (|CallParentFunction DeltaSeconds)
  (if (> (+ (Utilities|Array|Length (Collision|GetOverlappingActors (Variables|Default|GetCylinder) "/Game/Blueprints/BP_BaseCharacter.BP_BaseCharacter_C" :!class /Script/Engine.PrimitiveComponent)) (Utilities|Array|Length (Collision|GetOverlappingActors (Variables|Default|GetCylinder) "/Game/Blueprints/LevelBuild/BP_HeavyCube.BP_HeavyCube_C" :!class /Script/Engine.PrimitiveComponent))) 0)
    (Variables|Default|SetActive true)
    (Transformation|SetRelativeLocation _button (Math|Vector|MakeVector 0.0 0.0 (Math|Float|Clamp(Float) (- (.z _relativelocation) _returnvalue) -15.0 -4.0)) false false)
    (else
      (Variables|Default|SetActive false)
      (Transformation|SetRelativeLocation _button (Math|Vector|MakeVector 0.0 0.0 (Math|Float|Clamp(Float) (+ (.z _relativelocation) _returnvalue) -15.0 -4.0)) false false))))

(fn ConstructionScript
  (|CallParentFunction))