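; BP_Button is a level-building button that shows its timed active state as a countdown on four text renders.
; Each Tick decrements ActiveCountdown, clamping it at zero and clearing Active when it runs out; activation is not handled in these graphs.
; The Construction Script previews ActiveTIme on the same texts.
; Both graphs show whole numbers from ten upward and at zero, and one decimal otherwise.
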(event EventBeginPlay
  (|CallParentFunction) ; This node is disabled and will not be called.\nDrag off pins to build functionality.
)

(event Collision|EventActorBeginOverlap
  (params (OtherActor :type Actor%20Object%20Reference))
  (|CallParentFunction OtherActor) ; This node is disabled and will not be called.\nDrag off pins to build functionality.
)

(event EventTick
  (params (DeltaSeconds :type Float%20%28single-precision%29))
  (bind _textrender (Variables|Default|GetTextRender))
  (|CallParentFunction DeltaSeconds)
  (bind _output_get (Variables|Default|SetActiveCountdown (- (Variables|Default|GetActiveCountdown) DeltaSeconds)))
  (if (<= _output_get 0.0)
    (Variables|Default|SetActiveCountdown 0.0)
    (Variables|Default|SetActive false))
  (if (>= (Variables|Default|GetActiveCountdown) 1e+01)
    (Rendering|Components|TextRender|SetText _textrender (Utilities|Text|ToText(Float) (Variables|Default|GetActiveCountdown) "HalfToEven" true 1 2 0 0))
    (elif (!= (Variables|Default|GetActiveCountdown) 0.0)
      (Rendering|Components|TextRender|SetText _textrender (Utilities|Text|ToText(Float) (Variables|Default|GetActiveCountdown) "HalfToEven" true 1 2 1 1))
      (else
        (Rendering|Components|TextRender|SetText _textrender (Utilities|Text|ToText(Float) (Variables|Default|GetActiveCountdown) "HalfToEven" true 1 2 0 0))))))

(fn ConstructionScript
  (bind _textrender (Variables|Default|GetTextRender))
  (bind _activetime (Variables|Default|GetActiveTIme))
  (|CallParentFunction)
  (if (>= _activetime 1e+01)
    (Rendering|Components|TextRender|SetText _textrender (Utilities|Text|ToText(Float) _activetime "HalfToEven" true 1 2 0 0))
    (elif (!= _activetime 0.0)
      (Rendering|Components|TextRender|SetText _textrender (Utilities|Text|ToText(Float) _activetime "HalfToEven" true 1 2 1 1))
      (else
        (Rendering|Components|TextRender|SetText _textrender (Utilities|Text|ToText(Float) _activetime "HalfToEven" true 1 2 0 0))))))