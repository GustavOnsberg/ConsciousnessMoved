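; Plasma wall hazard of five stacked beam particles that kills the player and destroys heavy cubes on contact.
; Construction script and BeginPlay each place the beams and set their source and target points from Width.
; The wall is live when Active equals Inverse, which Tick uses to toggle beam visibility.
; While live, box overlap by any BP_BaseCharacter calls Die on player controller 0, and BP_HeavyCube actors are destroyed.
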(event OnComponentBeginOverlap(Box)
  (params (OverlappedComponent :type Primitive%20Component%20Object%20Reference) (OtherActor :type Actor%20Object%20Reference) (OtherComp :type Primitive%20Component%20Object%20Reference) (OtherBodyIndex :type Integer) (bFromSweep :type Boolean) (SweepResult :type Hit%20Result%20Structure%20%28by%20ref%29))
  (if (Math|Boolean|Equal(Boolean) (Variables|Default|GetActive) (Variables|Default|GetInverse))
    (Utilities|Casting|CastToBP_BaseCharacter OtherActor
      (:then
        (bind _asbp_player_controller (Utilities|Casting|CastToBP_PlayerController (Game|GetPlayerController 0)))
        (Default|Die _asbp_player_controller))
      (:CastFailed
        (bind _asbp_heavy_cube (Utilities|Casting|CastToBP_HeavyCube OtherActor))
        (Actor|DestroyActor _asbp_heavy_cube)))))

(event EventBeginPlay
  (|CallParentFunction)
  (CallFunction|SetParticleSourceandTarget))

(event Collision|EventActorBeginOverlap
  (params (OtherActor :type Actor%20Object%20Reference))
  (|CallParentFunction OtherActor) ; This node is disabled and will not be called.\nDrag off pins to build functionality.
)

(event EventTick
  (params (DeltaSeconds :type Float%20%28single-precision%29))
  (|CallParentFunction DeltaSeconds)
  (if (Math|Boolean|Equal(Boolean) (Variables|Default|GetActive) (Variables|Default|GetInverse))
    (Rendering|SetVisibility (Variables|Default|GetParticleSystem2) true false)
    (Variables|Default|SetEmitterEnabled true)
    (elif (Variables|Default|GetEmitterEnabled)
      (Rendering|SetVisibility (Variables|Default|GetParticleSystem) false false)
      (Variables|Default|SetEmitterEnabled false))))

(fn ConstructionScript
  (bind _particlesystem3 (Variables|Default|GetParticleSystem3))
  (bind _particlesystem4 (Variables|Default|GetParticleSystem4))
  (bind _particlesystem1 (Variables|Default|GetParticleSystem1))
  (bind _particlesystem2 (Variables|Default|GetParticleSystem2))
  (bind _particlesystem (Variables|Default|GetParticleSystem))
  (bind _returnvalue (Transformation|GetWorldLocation _particlesystem2))
  (bind _returnvalue_2 (Transformation|GetWorldLocation _particlesystem))
  (bind _returnvalue_3 (Transformation|GetWorldLocation _particlesystem3))
  (bind _returnvalue_4 (Transformation|GetWorldLocation _particlesystem4))
  (bind _returnvalue_5 (Transformation|GetWorldLocation _particlesystem1))
  (|CallParentFunction)
  (Transformation|SetRelativeLocation _particlesystem (Math|Vector|MakeVector (- 0.0 (/ (Variables|Default|GetWidth) 2.0)) 0.0 66.669998) false false)
  (Class|ParticleSystemComponent|SetBeamSourcePoint _particlesystem 0 _returnvalue_2)
  (Class|ParticleSystemComponent|SetBeamTargetPoint _particlesystem 0 (+ _returnvalue_2 (* (Math|Vector|GetForwardVector _particlesystem) (Variables|Default|GetWidth))))
  (Transformation|SetRelativeLocation _particlesystem1 (Math|Vector|MakeVector (- 0.0 (/ (Variables|Default|GetWidth) 2.0)) 0.0 133.339996) false false)
  (Class|ParticleSystemComponent|SetBeamSourcePoint _particlesystem1 0 _returnvalue_5)
  (Class|ParticleSystemComponent|SetBeamTargetPoint _particlesystem1 0 (+ _returnvalue_5 (* (Math|Vector|GetForwardVector _particlesystem1) (Variables|Default|GetWidth))))
  (Transformation|SetRelativeLocation _particlesystem2 (Math|Vector|MakeVector (- 0.0 (/ (Variables|Default|GetWidth) 2.0)) 0.0 2e+02) false false)
  (Class|ParticleSystemComponent|SetBeamSourcePoint _particlesystem2 0 _returnvalue)
  (Class|ParticleSystemComponent|SetBeamTargetPoint _particlesystem2 0 (+ _returnvalue (* (Math|Vector|GetForwardVector _particlesystem2) (Variables|Default|GetWidth))))
  (Transformation|SetRelativeLocation _particlesystem3 (Math|Vector|MakeVector (- 0.0 (/ (Variables|Default|GetWidth) 2.0)) 0.0 266.670013) false false)
  (Class|ParticleSystemComponent|SetBeamSourcePoint _particlesystem3 0 _returnvalue_3)
  (Class|ParticleSystemComponent|SetBeamTargetPoint _particlesystem3 0 (+ _returnvalue_3 (* (Math|Vector|GetForwardVector _particlesystem3) (Variables|Default|GetWidth))))
  (Transformation|SetRelativeLocation _particlesystem4 (Math|Vector|MakeVector (- 0.0 (/ (Variables|Default|GetWidth) 2.0)) 0.0 333.339996) false false)
  (Class|ParticleSystemComponent|SetBeamSourcePoint _particlesystem4 0 _returnvalue_4)
  (Class|ParticleSystemComponent|SetBeamTargetPoint _particlesystem4 0 (+ _returnvalue_4 (* (Math|Vector|GetForwardVector _particlesystem4) (Variables|Default|GetWidth)))))

(fn SetParticleSourceandTarget
  (bind _particlesystem3 (Variables|Default|GetParticleSystem3))
  (bind _particlesystem4 (Variables|Default|GetParticleSystem4))
  (bind _particlesystem1 (Variables|Default|GetParticleSystem1))
  (bind _particlesystem2 (Variables|Default|GetParticleSystem2))
  (bind _particlesystem (Variables|Default|GetParticleSystem))
  (bind _returnvalue (Transformation|GetWorldLocation _particlesystem2))
  (bind _returnvalue_2 (Transformation|GetWorldLocation _particlesystem))
  (bind _returnvalue_3 (Transformation|GetWorldLocation _particlesystem3))
  (bind _returnvalue_4 (Transformation|GetWorldLocation _particlesystem4))
  (bind _returnvalue_5 (Transformation|GetWorldLocation _particlesystem1))
  (Transformation|SetRelativeLocation _particlesystem (Math|Vector|MakeVector (- 0.0 (/ (Variables|Default|GetWidth) 2.0)) 0.0 66.669998) false false)
  (Class|ParticleSystemComponent|SetBeamSourcePoint _particlesystem 0 _returnvalue_2)
  (Class|ParticleSystemComponent|SetBeamTargetPoint _particlesystem 0 (+ _returnvalue_2 (* (Math|Vector|GetForwardVector _particlesystem) (Variables|Default|GetWidth))))
  (Transformation|SetRelativeLocation _particlesystem1 (Math|Vector|MakeVector (- 0.0 (/ (Variables|Default|GetWidth) 2.0)) 0.0 133.339996) false false)
  (Class|ParticleSystemComponent|SetBeamSourcePoint _particlesystem1 0 _returnvalue_5)
  (Class|ParticleSystemComponent|SetBeamTargetPoint _particlesystem1 0 (+ _returnvalue_5 (* (Math|Vector|GetForwardVector _particlesystem1) (Variables|Default|GetWidth))))
  (Transformation|SetRelativeLocation _particlesystem2 (Math|Vector|MakeVector (- 0.0 (/ (Variables|Default|GetWidth) 2.0)) 0.0 2e+02) false false)
  (Class|ParticleSystemComponent|SetBeamSourcePoint _particlesystem2 0 _returnvalue)
  (Class|ParticleSystemComponent|SetBeamTargetPoint _particlesystem2 0 (+ _returnvalue (* (Math|Vector|GetForwardVector _particlesystem2) (Variables|Default|GetWidth))))
  (Transformation|SetRelativeLocation _particlesystem3 (Math|Vector|MakeVector (- 0.0 (/ (Variables|Default|GetWidth) 2.0)) 0.0 266.670013) false false)
  (Class|ParticleSystemComponent|SetBeamSourcePoint _particlesystem3 0 _returnvalue_3)
  (Class|ParticleSystemComponent|SetBeamTargetPoint _particlesystem3 0 (+ _returnvalue_3 (* (Math|Vector|GetForwardVector _particlesystem3) (Variables|Default|GetWidth))))
  (Transformation|SetRelativeLocation _particlesystem4 (Math|Vector|MakeVector (- 0.0 (/ (Variables|Default|GetWidth) 2.0)) 0.0 333.339996) false false)
  (Class|ParticleSystemComponent|SetBeamSourcePoint _particlesystem4 0 _returnvalue_4)
  (Class|ParticleSystemComponent|SetBeamTargetPoint _particlesystem4 0 (+ _returnvalue_4 (* (Math|Vector|GetForwardVector _particlesystem4) (Variables|Default|GetWidth)))))