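; BP_LaserCube is a laser emitter actor that fires a beam along its cube's forward vector and feeds laser receivers.
; Each tick, a long Visibility line trace looks for a BP_LaserReciver, stores it as LaserTarget and adds itself to that receiver's LaserOrigins, otherwise clearing the target.
; The particle beam is then stretched from the particle system's location to the trace impact point.
; It never removes itself from LaserOrigins.
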(event EventBeginPlay
  (|CallParentFunction) ; This node is disabled and will not be called.\nDrag off pins to build functionality.
)

(event Collision|EventActorBeginOverlap
  (params (OtherActor :type Actor%20Object%20Reference))
  (|CallParentFunction OtherActor) ; This node is disabled and will not be called.\nDrag off pins to build functionality.
)

(event EventTick
  (params (DeltaSeconds :type Float%20%28single-precision%29))
  (bind _particlesystem (Variables|Default|GetParticleSystem))
  (bind _cube (Variables|Default|GetCube))
  (bind _returnvalue (Transformation|GetWorldLocation _cube))
  (|CallParentFunction DeltaSeconds)
  (bind _outhit (Collision|LineTraceByChannel _returnvalue (+ _returnvalue (* (Math|Vector|GetForwardVector _cube) 2e+04)) "TraceTypeQuery1" false 0 "None"))
  (bind _asbp_laser_reciver (Utilities|Casting|CastToBP_LaserReciver (.HitActor (Collision|BreakHitResult _outhit)))
    (:then
      (Variables|Default|SetLaserTarget _asbp_laser_reciver)
      (Utilities|Array|AddUnique (Variables|/Game/Blueprints/LevelBuild/BP_LaserReciver.BP_LaserReciver_C|GetLaserOrigins _asbp_laser_reciver) self))
    (:CastFailed
      (Variables|Default|SetLaserTarget 0)))
  (Class|ParticleSystemComponent|SetBeamSourcePoint _particlesystem 0 (Transformation|GetWorldLocation _particlesystem))
  (Class|ParticleSystemComponent|SetBeamTargetPoint _particlesystem 0 (.ImpactPoint (Collision|BreakHitResult _outhit))))

(fn ConstructionScript
  (|CallParentFunction))