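; BP_HeavyCube is a physics cube that can be carried and that floats along anti-gravity fields.
; Each Tick, a carried cube drops gravity, chases the carrier's CarryPosition by setting velocity and eases its rotation toward the carrier's.
; Otherwise, a current anti-gravity field replaces gravity with heavy angular damping and a velocity along the field's up vector, corrected toward its axis.
; With neither, normal gravity and zero angular damping return.
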(event EventBeginPlay)

(event Collision|EventActorBeginOverlap
  (params (OtherActor :type Actor%20Object%20Reference)))

(event EventTick
  (params (DeltaSeconds :type Float%20%28single-precision%29))
  (bind _carriedby (Variables|Default|GetCarriedBy))
  (bind _cube (Variables|Default|GetCube))
  (bind _cube_2 (Variables|Default|GetCube))
  (bind _cube_3 (Variables|Default|GetCube))
  (bind _currentantigravityfield (Variables|Default|GetCurrentAntiGravityField))
  (bind _returnvalue (Transformation|GetWorldLocation _cube_2))
  (bind _returnvalue_2 (Transformation|GetActorUpVector _currentantigravityfield))
  (bind _returnvalue_3 (Transformation|GetActorLocation _currentantigravityfield))
  (bind _returnvalue_4 (- _returnvalue_3 _returnvalue))
  (if (Variables|Default|GetIsCarried)
    (Physics|SetEnableGravity _cube false)
    (Physics|SetPhysicsLinearVelocity _cube (* (- (Transformation|GetWorldLocation (Variables|/Game/Blueprints/BP_BaseCharacter.BP_BaseCharacter_C|GetCarryPosition _carriedby)) (Transformation|GetWorldLocation _cube)) 1e+01) false "None")
    (Class|PrimitiveComponent|SetAngularDamping _cube 1e+01)
    (Transformation|SetWorldRotation _cube (Math|Rotator|Lerp(Rotator) (Transformation|GetWorldRotation _cube) (Transformation|GetActorRotation _carriedby) (* DeltaSeconds 1e+01) true) false false)
    (elif (== (Variables|Default|GetCurrentAntiGravityField) 0)
      (Physics|SetEnableGravity _cube true)
      (Class|PrimitiveComponent|SetAngularDamping _cube 0.0)
      (else
        (Physics|SetEnableGravity _cube_3 false)
        (Class|PrimitiveComponent|SetAngularDamping _cube_3 5e+01)
        (Physics|SetPhysicsLinearVelocity _cube_3 (- (* _returnvalue_2 2e+02) (* (- (- (Transformation|GetWorldLocation (Variables|Default|GetCube)) (* _returnvalue_2 (Math|Float|Sqrt (+ (Math|Float|Square (.x _returnvalue_4)) (Math|Float|Square (.y _returnvalue_4)) (Math|Float|Square (.z _returnvalue_4)))))) (Transformation|GetActorLocation _currentantigravityfield)) 0.6)) false "None")))))

(fn ConstructionScript)