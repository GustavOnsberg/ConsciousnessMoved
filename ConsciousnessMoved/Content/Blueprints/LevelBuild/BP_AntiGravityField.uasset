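; BP_AntiGravityField is a switchable level field with Off, Push and Pull states for heavy cubes and characters.
; Each tick, Active selects the configured active or inactive status, which sets the mesh's visibility and material.
; While visible, a line trace along the actor's up vector stretches the field to the hit distance.
; Mesh overlaps set or clear CurrentAntiGravityField on BP_HeavyCube and BP_BaseCharacter; no force is applied here.
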(event OnComponentBeginOverlap(FieldMesh)
  (params (OverlappedComponent :type Primitive%20Component%20Object%20Reference) (OtherActor :type Actor%20Object%20Reference) (OtherComp :type Primitive%20Component%20Object%20Reference) (OtherBodyIndex :type Integer) (bFromSweep :type Boolean) (SweepResult :type Hit%20Result%20Structure%20%28by%20ref%29))
  (bind _self self)
  (bind _asbp_heavy_cube (Utilities|Casting|CastToBP_HeavyCube OtherActor)
    (:then
      (Variables|/Game/Blueprints/LevelBuild/BP_HeavyCube.BP_HeavyCube_C|SetCurrentAntiGravityField _asbp_heavy_cube _self))
    (:CastFailed
      (bind _asbp_base_character (Utilities|Casting|CastToBP_BaseCharacter OtherActor))
      (Variables|/Game/Blueprints/BP_BaseCharacter.BP_BaseCharacter_C|SetCurrentAntiGravityField _asbp_base_character _self))))

(event OnComponentEndOverlap(FieldMesh)
  (params (OverlappedComponent :type Primitive%20Component%20Object%20Reference) (OtherActor :type Actor%20Object%20Reference) (OtherComp :type Primitive%20Component%20Object%20Reference) (OtherBodyIndex :type Integer))
  (bind _self self)
  (bind _asbp_heavy_cube (Utilities|Casting|CastToBP_HeavyCube OtherActor)
    (:then
      (if (== _self (Variables|/Game/Blueprints/LevelBuild/BP_HeavyCube.BP_HeavyCube_C|GetCurrentAntiGravityField _asbp_heavy_cube))
        (Variables|/Game/Blueprints/LevelBuild/BP_HeavyCube.BP_HeavyCube_C|SetCurrentAntiGravityField _asbp_heavy_cube 0)))
    (:CastFailed
      (bind _asbp_base_character (Utilities|Casting|CastToBP_BaseCharacter OtherActor))
      (if (== _self (Variables|/Game/Blueprints/BP_BaseCharacter.BP_BaseCharacter_C|GetCurrentAntiGravityField _asbp_base_character))
        (Variables|/Game/Blueprints/BP_BaseCharacter.BP_BaseCharacter_C|SetCurrentAntiGravityField _asbp_base_character 0)))))

(event EventBeginPlay
  (|CallParentFunction) ; This node is disabled and will not be called.\nDrag off pins to build functionality.
)

(event Collision|EventActorBeginOverlap
  (params (OtherActor :type Actor%20Object%20Reference))
  (|CallParentFunction OtherActor) ; This node is disabled and will not be called.\nDrag off pins to build functionality.
)

(event EventTick
  (params (DeltaSeconds :type Float%20%28single-precision%29))
  (bind _returnvalue (Transformation|GetActorLocation))
  (bind _fieldmesh (Variables|Default|GetFieldMesh))
  (|CallParentFunction DeltaSeconds)
  (Utilities|FlowControl|Sequence
    (:then_0
      (if (Variables|Default|GetActive)
        (Variables|Default|SetCurrentStatus (Variables|Default|GetActiveStatus))
        (else
          (Variables|Default|SetCurrentStatus (Variables|Default|GetInactiveStatus))))
      (switch Utilities|FlowControl|Switch|SwitchonAntiGravityFieldStatus (Variables|Default|GetCurrentStatus)
        (:NewEnumerator0
          (Rendering|SetVisibility _fieldmesh false false))
        (:NewEnumerator1
          (Rendering|Material|SetMaterial _fieldmesh 0 "/Game/Materials/Mat_AntiGravityField_Push.Mat_AntiGravityField_Push")
          (Rendering|SetVisibility _fieldmesh true false :!label _label)
          (bind _outhit (Collision|LineTraceByChannel _returnvalue (+ _returnvalue (* (Transformation|GetActorUpVector) 1e+04)) "TraceTypeQuery3" false 0 "None"))
          (Transformation|SetRelativeScale3D (Variables|Default|GetField) (Math|Vector|MakeVector 1.0 1.0 (+ (/ (.Distance (Collision|BreakHitResult _outhit)) 1e+02) 0.1))))
        (:NewEnumerator2
          (Rendering|Material|SetMaterial _fieldmesh 0 "/Game/Materials/Mat_AntiGravityField_Pull.Mat_AntiGravityField_Pull")
          (goto _label))))))

(fn ConstructionScript
  (|CallParentFunction))