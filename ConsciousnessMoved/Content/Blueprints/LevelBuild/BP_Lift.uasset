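; BP_Lift is a lift actor that moves its Platform component vertically between its base and a configurable Height.
; Every Tick steps the platform's relative Z by Speed times delta time, clamped to that range.
; Active sends it up and inactive sends it down, with Inverted swapping those directions.
; The graph only reads Active and never sets it.
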(event EventBeginPlay
  (|CallParentFunction) ; This node is disabled and will not be called.\nDrag off pins to build functionality.
)

(event Collision|EventActorBeginOverlap
  (params (OtherActor :type Actor%20Object%20Reference))
  (|CallParentFunction OtherActor) ; This node is disabled and will not be called.\nDrag off pins to build functionality.
)

(event EventTick
  (params (DeltaSeconds :type Float%20%28single-precision%29))
  (bind _inverted (Variables|Default|GetInverted))
  (bind _platform (Variables|Default|GetPlatform))
  (bind _speed (Variables|Default|GetSpeed))
  (bind _returnvalue (* DeltaSeconds _speed))
  (bind _relativelocation (Variables|/Script/Engine.SceneComponent|GetRelativeLocation _platform))
  (|CallParentFunction DeltaSeconds)
  (if (Variables|Default|GetActive)
    (if _inverted
      (Transformation|SetRelativeLocation _platform (Math|Vector|MakeVector 0.0 0.0 (Math|Float|Clamp(Float) (- (.z _relativelocation) _returnvalue) 0.0 (Variables|Default|GetHeight))) false false :!label _label)
      (else
        (Transformation|SetRelativeLocation _platform (Math|Vector|MakeVector 0.0 0.0 (Math|Float|Clamp(Float) (+ (.z _relativelocation) _returnvalue) 0.0 (Variables|Default|GetHeight))) false false :!label _label_2)))
    (elif _inverted
      (goto _label_2)
      (else
        (goto _label)))))

(fn ConstructionScript
  (|CallParentFunction))