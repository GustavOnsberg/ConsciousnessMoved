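; BP_PowerLine is a spline-shaped power line that shows an on or off state with beam particle effects.
; The construction script creates a particle component per spline point, defaulting to the off template, with each beam running from its point to the next in world space.
; BeginPlay reapplies those beam endpoints.
; SetIsOn swaps every component's template between on and off, then reruns the same endpoint update.
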(event Custom|SetIsOn
  (params (IsOn :type Boolean))
  (bind _particlesystems (Variables|Default|GetParticleSystems))
  (bind _spline (Variables|Default|GetSpline))
  (if IsOn
    (Effects|Components|ParticleSystem|SetTemplate _particlesystems "/Game/Particle/PS_PowerLine_On.PS_PowerLine_On")
    (else
      (Effects|Components|ParticleSystem|SetTemplate _particlesystems "/Game/Particle/PS_PowerLine_Off.PS_PowerLine_Off")))
  (for _index (range 0 (Spline|GetNumberOfSplinePoints _spline))
    (Class|ParticleSystemComponent|SetBeamTargetPoint (Utilities|Array|Get(acopy) (Variables|Default|GetParticleSystems) _index) 0 (Spline|GetLocationatSplinePoint _spline (+ _index 1) "World"))
    (Class|ParticleSystemComponent|SetBeamSourcePoint (Utilities|Array|Get(acopy) (Variables|Default|GetParticleSystems) _index) 0 (Spline|GetLocationatSplinePoint _spline _index "World"))))

(event EventBeginPlay
  (bind _spline (Variables|Default|GetSpline))
  (for _index (range 0 (Spline|GetNumberOfSplinePoints _spline))
    (Class|ParticleSystemComponent|SetBeamTargetPoint (Utilities|Array|Get(acopy) (Variables|Default|GetParticleSystems) _index) 0 (Spline|GetLocationatSplinePoint _spline (+ _index 1) "World"))
    (Class|ParticleSystemComponent|SetBeamSourcePoint (Utilities|Array|Get(acopy) (Variables|Default|GetParticleSystems) _index) 0 (Spline|GetLocationatSplinePoint _spline _index "World"))))

(event Collision|EventActorBeginOverlap
  (params (OtherActor :type Actor%20Object%20Reference)))

(event EventTick
  (params (DeltaSeconds :type Float%20%28single-precision%29)))

(fn ConstructionScript
  (bind _spline (Variables|Default|GetSpline))
  (while (> (Utilities|Array|Length (Variables|Default|GetParticleSystems)) 0)
    (Components|DestroyComponent (Utilities|Array|Get(acopy) (Variables|Default|GetParticleSystems))))
  (for _index (range 0 (Spline|GetNumberOfSplinePoints _spline))
    (bind _returnvalue (AddComponent|AddParticleSystemComponent false))
    (Utilities|Array|Add (Variables|Default|GetParticleSystems) _returnvalue)
    (Effects|Components|ParticleSystem|SetTemplate _returnvalue "/Game/Particle/PS_PowerLine_Off.PS_PowerLine_Off")
    (Class|ParticleSystemComponent|SetBeamTargetPoint _returnvalue 0 (Spline|GetLocationatSplinePoint _spline (+ _index 1) "World"))
    (Class|ParticleSystemComponent|SetBeamSourcePoint _returnvalue 0 (Spline|GetLocationatSplinePoint _spline _index "World"))))