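; Laser receiver actor that detects when a laser is targeting it and shows that state with a colored light.
; Each Tick it polls LaserOrigins, casts entries to BP_Laser_Character, and sets Active when one has this actor as LasarTarget, stopping at the first match.
; The Light then turns green when Active and red otherwise.
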(event EventBeginPlay
  (|CallParentFunction) ; This node is disabled and will not be called.\nDrag off pins to build functionality.
)

(event Collision|EventActorBeginOverlap
  (params (OtherActor :type Actor%20Object%20Reference))
  (|CallParentFunction OtherActor) ; This node is disabled and will not be called.\nDrag off pins to build functionality.
)

(event EventTick
  (params (DeltaSeconds :type Float%20%28single-precision%29))
  (bind _light (Variables|Default|GetLight))
  (|CallParentFunction DeltaSeconds)
  (bind _array_element (Utilities|Array|ForEachLoopwithBreak (Variables|Default|GetLaserOrigins) :!label _label)
    (:LoopBody
      (bind _asbp_laser_character (Utilities|Casting|CastToBP_Laser_Character _array_element))
      (if (== (Variables|/Game/Blueprints/Characters/BP_Laser_Character.BP_Laser_Character_C|GetLasarTarget _asbp_laser_character) self)
        (Variables|Default|SetActive true)
        (goto _label Break)
        (else
          (Variables|Default|SetActive false))))
    (:Completed
      (if (Variables|Default|GetActive)
        (Rendering|Components|Light|SetLightColor _light "(R=0.000000,G=1.000000,B=0.000000,A=1.000000)" true)
        (else
          (Rendering|Components|Light|SetLightColor _light "(R=1.000000,G=0.000000,B=0.000000,A=1.000000)" true))))))

(fn ConstructionScript
  (|CallParentFunction))