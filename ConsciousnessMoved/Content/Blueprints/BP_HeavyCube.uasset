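; BP_HeavyCube is a physics cube that a carrier can hold and move.
; While IsCarried is set, Tick disables gravity and drives linear velocity toward the carrier's CarryPosition, proportional to the remaining distance.
; It also raises angular damping and smoothly rotates the cube to match the carrier's rotation.
; When not carried, gravity is restored and angular damping cleared; carry state is not assigned in this Blueprint.
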(event EventBeginPlay)

(event Collision|EventActorBeginOverlap
  (params (OtherActor :type Actor%20Object%20Reference)))

(event EventTick
  (params (DeltaSeconds :type Float%20%28single-precision%29))
  (bind _carriedby (Variables|Default|GetCarriedBy))
  (bind _cube (Variables|Default|GetCube))
  (if (Variables|Default|GetIsCarried)
    (Physics|SetEnableGravity _cube false)
    (Physics|SetPhysicsLinearVelocity _cube (* (- (Transformation|GetWorldLocation (Variables|/Game/Blueprints/BP_BaseCharacter.BP_BaseCharacter_C|GetCarryPosition _carriedby)) (Transformation|GetWorldLocation _cube)) 1e+01) false "None")
    (Class|PrimitiveComponent|SetAngularDamping _cube 1e+01)
    (Transformation|SetWorldRotation _cube (Math|Rotator|Lerp(Rotator) (Transformation|GetWorldRotation _cube) (Transformation|GetActorRotation _carriedby) (* DeltaSeconds 1e+01) true) false false)
    (else
      (Physics|SetEnableGravity _cube true)
      (Class|PrimitiveComponent|SetAngularDamping _cube 0.0))))

(fn ConstructionScript)